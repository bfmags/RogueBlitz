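; Blackhole projectile that destroys simulating actors (BP_SimulatingActor) touching its Sphere component.
; On BeginPlay it makes SphereComp ignore the instigator while moving and binds the Sphere's begin-overlap event.
; Overlapping actors are destroyed immediately if their class exactly matches BP_SimulatingActor.
; A one-shot timer destroys the projectile itself after a few seconds.
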(event Custom|DestriyActor
  (Actor|DestroyActor))

(event Custom|OnComponentBeginOverlap_Event
  (params (OverlappedComponent :type Primitive%20Component%20Object%20Reference) (OtherActor :type Actor%20Object%20Reference) (OtherComp :type Primitive%20Component%20Object%20Reference) (OtherBodyIndex :type Integer) (bFromSweep :type Boolean) (SweepResult :type Hit%20Result%20Structure%20%28by%20ref%29))
  ;[0 0 0] Add to list to be shrunk and destroyed
  (Utilities|IsValid OtherActor
    (:Is%20Valid
      (if (== (Utilities|GetClass OtherActor) "/Game/RogueBlitz/Blueprints/BP_SimulatingActor.BP_SimulatingActor_C")
        (Actor|DestroyActor OtherActor)))))

(event EventBeginPlay
  (Collision|IgnoreActorwhenMoving (Variables|Default|GetSphereComp) (Game|GetInstigator) true)
  (Utilities|Time|SetTimerbyEvent (delegate Custom|DestriyActor) 5.0)
  ;[0 0 0] Add to list to be shrunk and destroyed
  (Collision|AssignOnComponentBeginOverlap (Variables|Default|GetSphere) (delegate Custom|OnComponentBeginOverlap_Event)))

(fn ConstructionScript)