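; BP_CannonChair is a turret actor that tracks the first player's pawn and fires magic projectiles at it.
; Tick turns the root's yaw toward the player with a -90 degree offset, so the local Y axis faces the target.
; A looping timer started on BeginPlay spawns BP_MagicProjectile at the actor's transform and launches it along that local Y axis.
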(event Custom|FireCannon
  (bind _returnvalue (Game|SpawnActorfromClass "/Game/RogueBlitz/BP_MagicProjectile.BP_MagicProjectile_C" (Math|Transform|MakeTransform (Transformation|GetActorLocation) (Transformation|GetActorRotation) "1.000000,1.000000,1.000000") "AlwaysSpawn" "MultiplyWithRoot" 0 self))
  (Game|Components|ProjectileMovement|SetVelocityinLocalSpace (Variables|/Script/RogueBlitz.RBMagicProjectile|GetMovementComp _returnvalue) "0.000000,1000.000000,0.000000"))

(event EventBeginPlay
  (Utilities|Time|SetTimerbyEvent (delegate Custom|FireCannon) 2.0 true))

(event EventTick
  (params (DeltaSeconds :type Float%20%28single-precision%29))
  (Transformation|SetWorldRotation (Variables|Default|GetDefaultSceneRoot self) (Math|Rotator|MakeRotator 0.0 0.0 (+ (.yaw (Math|Rotator|FindLookatRotation (Transformation|GetActorLocation) (Transformation|GetActorLocation (Game|Player|GetPlayerPawn 0)))) -9e+01)) false false))

(fn ConstructionScript)